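; Visual actor for an EMF device with hull, pipes, magnet internals and Niagara particles, animated through Sequencer-callable events.
; Construction creates hull and inner-structure dynamic materials and sets particle separation parameters.
; Events toggle particles and indicators, while timelines ramp particle time dilation and hull translucency.
; FadeOutHull only stores values because its update is disconnected, and PipeWaterFlow's material instance creation is also unwired.
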(event Custom|PipeWaterFlow
  (params (FlowSpeed :type Float%20%28single-precision%29))
  (Rendering|Material|SetScalarParameterValue (Variables|Default|GetDMI_PipeFlow) "Speed" FlowSpeed :!class /Script/Engine.MaterialInstanceDynamic))

(event Custom|AnimatHullTranslucecy
  (params (FadeOutTime :type Float%20%28single-precision%29))
  (bind _newtrack_0 (Timeline|Timeline_0 Play)
    (:Update
      (Rendering|Material|SetScalarParameterValue (Variables|EMFOuterDMI|GetDMI_EMF_Hull) "Trans" _newtrack_0 :!class /Script/Engine.MaterialInstanceDynamic))))

(event Custom|FadeOutHull
  (params (Time :type Float%20%28single-precision%29) (HullOpacityPercentageFrom :type Float%20%28single-precision%29) (HullOpacityPercentageTo :type Float%20%28single-precision%29) (HullOutlineOpacityPercentageFrom :type Float%20%28single-precision%29) (HullOutlineOpacityPercentageTo :type Float%20%28single-precision%29))
  (Variables|Default|SetIsFadeoutHull true)
  (Variables|Default|SetFadeOutTime Time)
  (Utilities|FlowControl|Sequence
    (:then_0
      (Variables|Default|SetFadeOutHullPercentageFrom HullOpacityPercentageFrom)
      (Variables|Default|SetFadeOutHullPercentageTo HullOpacityPercentageTo))
    (:then_1
      (Variables|Default|SetFadeOutHullOutlinePercentageFrom HullOutlineOpacityPercentageFrom)
      (Variables|Default|SetFadeOutHullOutlinePercentageTo HullOutlineOpacityPercentageTo))))

(event Custom|EditorDebugSetVisibility
  ;[1 1 1] 编辑器上的方便显隐物体函数
  (Rendering|SetVisibility (Variables|Default|GetMainStruct) (Variables|Default|GetShowMainStruct) false)
  (Rendering|SetVisibility (Variables|Default|GetPipes) (Variables|Default|GetShowPipe) false)
  (Rendering|SetVisibility (Variables|Default|GetPipeFlow) (Variables|Default|GetShowPipeFlow) false)
  (Rendering|SetVisibility (Variables|Default|GetBolts1) (Variables|Default|GetShowBolt) false)
  (Rendering|SetVisibility (Variables|Default|GetInnerStruct) (Variables|Default|GetShowInner) false))

(event Custom|SetParticleTimeDilation
  (Niagara|SetNiagaraVariable(Float) (Variables|Default|GetNiagara) "User.CustomTimeDIalition" (Variables|ParticleControl|GetP_CustomTimeDilation)))

(event Custom|ToggleParticleVisibility
  (params (IsShow :type Boolean))
  ;[1 1 1] 响应Sequencer的事件调用
  (Rendering|SetVisibility (Variables|Default|GetNiagara) IsShow false))

(event Custom|MakeParticleAlive
  ;[1 1 1] 响应Sequencer的事件调用
  (bind _alpha (Timeline|Timeline_1 Play)
    (:Update
      (bind _output_get (Variables|ParticleControl|SetP_CustomTimeDilation (Math|Float|Lerp 0.0 1.0 _alpha)))
      (Niagara|SetNiagaraVariable(Float) (Variables|Default|GetNiagara) "User.CustomTimeDIalition" _output_get))))

(event Custom|ToggleLightIndicatorVis
  (params (IsShow :type Boolean))
  ;[1 1 1] 响应Sequencer的事件调用
  (Rendering|SetVisibility (Variables|Default|GetSM_EMF_LightIndicator) IsShow false))

(event Custom|ShowFlowMeshIndicator
  (Rendering|SetVisibility (Variables|Default|GetFlowMeshIndicator) true false))

(event EventBeginPlay
  ;[1 1 1] 开始的时候先让粒子发射器发射，暂时隐藏掉，等8秒停住，待到后面用seq显示
)

(event Collision|EventActorBeginOverlap
  (params (OtherActor :type Actor%20Object%20Reference)))

(event EventTick
  (params (DeltaSeconds :type Float%20%28single-precision%29)))

(event Input|KeyboardEvents|X
  (params (Key :type Key%20Structure)))

(event Input|KeyboardEvents|X
  (params (Key :type Key%20Structure))
  (:Pressed
    (Variables|ParticleControl|SetP_SperateLength 0.0))
  (:Released
    (Variables|ParticleControl|SetP_SperateLength 5e+01)))

(fn ConstructionScript
  (Utilities|FlowControl|Sequence
    (:then_0
      (CallFunction|CreateEMFDMI))
    (:then_1
      (CallFunction|CreateEMFIDMI))
    (:then_2
      (CallFunction|NiagaraUpdatePosition))
    (:then_3
      (CallFunction|NiagaraUpdateSperate 0.0))))

(fn CreateEMFDMI
  (Utilities|FlowControl|Sequence
    (:then_0
      (bind _returnvalue (Rendering|Material|CreateDynamicMaterialInstance (Variables|Default|GetMainStruct) 0 "/Game/MZConceptClass/EMF/Materials/MI_EMF_Hull.MI_EMF_Hull" "None" :!class /Script/Engine.PrimitiveComponent))
      (Variables|EMFOuterDMI|SetDMI_EMF_Hull _returnvalue))
    (:then_1
      (bind _returnvalue_2 (Rendering|Material|CreateDynamicMaterialInstance (Variables|Default|GetMainStruct) 1 "/Game/MZConceptClass/EMF/Materials/MI_EMF_Hull_Panel.MI_EMF_Hull_Panel" "None" :!class /Script/Engine.PrimitiveComponent))
      (Variables|EMFOuterDMI|SetDMI_EMF_Panel _returnvalue_2))
    (:then_2
      (bind _returnvalue_3 (Rendering|Material|CreateDynamicMaterialInstance (Variables|Default|GetMainStruct) 2 "/Game/MZConceptClass/EMF/Materials/MI_EMF_Hull_Bolt.MI_EMF_Hull_Bolt" "None" :!class /Script/Engine.PrimitiveComponent))
      (Variables|EMFOuterDMI|SetDMI_EMF_Bolt _returnvalue_3))
    (:then_3
      (bind _returnvalue_4 (Rendering|Material|CreateDynamicMaterialInstance (Variables|Default|GetMainStruct) 3 "/Game/MZConceptClass/EMF/Materials/MI_EMF_Hull_Inner.MI_EMF_Hull_Inner" "None" :!class /Script/Engine.PrimitiveComponent))
      (Variables|EMFOuterDMI|SetDMI_EMF_Inner _returnvalue_4))
    (:then_4
      (bind _returnvalue_5 (Rendering|Material|CreateDynamicMaterialInstance (Variables|Default|GetBolts1) 0 "/Game/MZConceptClass/EMF/Materials/MI_EMF_Hull_Bolt.MI_EMF_Hull_Bolt" "None" :!class /Script/Engine.PrimitiveComponent))
      (Variables|EMFOuterDMI|SetDMI_EMF_OutterBolt _returnvalue_5))
    (:then_5
      (bind _returnvalue_6 (Rendering|Material|CreateDynamicMaterialInstance (Variables|Default|GetPipes) 0 "/Game/MZConceptClass/EMF/Materials/MI_EMF_Hull_Bolt.MI_EMF_Hull_Bolt" "None" :!class /Script/Engine.PrimitiveComponent))
      (Variables|EMFOuterDMI|SetDMI_EMF_OutterPipe _returnvalue_6))))

(fn UpdateHullFadeOut
  (params (DeltaTime :type Float%20%28single-precision%29)))

(fn CreateEMFIDMI
  (bind _innerstruct (Variables|Default|GetInnerStruct))
  (Utilities|FlowControl|Sequence
    (:then_0
      (bind _returnvalue (Rendering|Material|CreateDynamicMaterialInstance _innerstruct 0 "/Game/MZConceptClass/EMF/Materials/MI_EMFI_TopMag.MI_EMFI_TopMag" "None" :!class /Script/Engine.PrimitiveComponent))
      (Variables|InnerStructDMI|SetDMI_EMFI_Top _returnvalue))
    (:then_1
      (bind _returnvalue_2 (Rendering|Material|CreateDynamicMaterialInstance _innerstruct 1 "/Game/MZConceptClass/EMF/Materials/MI_EMFI_BottomMag.MI_EMFI_BottomMag" "None" :!class /Script/Engine.PrimitiveComponent))
      (Variables|InnerStructDMI|SetDMI_EMFI_Bottom _returnvalue_2))
    (:then_2
      (bind _returnvalue_3 (Rendering|Material|CreateDynamicMaterialInstance _innerstruct 2 "/Game/MZConceptClass/EMF/Materials/MI_EMFI_InnerBolt.MI_EMFI_InnerBolt" "None" :!class /Script/Engine.PrimitiveComponent))
      (Variables|InnerStructDMI|SetDMI_EMFI_InnerBolt _returnvalue_3))
    (:then_3
      (bind _returnvalue_4 (Rendering|Material|CreateDynamicMaterialInstance _innerstruct 3 "/Game/MZConceptClass/EMF/Materials/MI_EMFI_FieldLine.MI_EMFI_FieldLine" "None" :!class /Script/Engine.PrimitiveComponent))
      (Variables|InnerStructDMI|SetDMI_EMFI_MagField _returnvalue_4))
    (:then_4
      (bind _returnvalue_5 (Rendering|Material|CreateDynamicMaterialInstance _innerstruct 4 "/Game/MZConceptClass/EMF/Materials/MI_EMFI_InnerShell.MI_EMFI_InnerShell" "None" :!class /Script/Engine.PrimitiveComponent))
      (Variables|InnerStructDMI|SetDMI_EMFI_InnerShell _returnvalue_5))))

(fn NiagaraUpdateSperate
  (params (DeltaTime :type Float%20%28single-precision%29))
  (bind _output_get (Variables|ParticleControl|SetP_Sperate 1.2e+02))
  (Niagara|SetNiagaraVariable(Float) (Variables|Default|GetNiagara) "User.Sperate" _output_get))

(fn NiagaraUpdatePosition
  (bind _niagara (Variables|Default|GetNiagara))
  (Niagara|SetNiagaraVariable(Float) _niagara "User.SperatePosition" (Variables|ParticleControl|GetP_SperatePosition))
  (Niagara|SetNiagaraVariable(Float) _niagara "User.SperateLength" (Variables|ParticleControl|GetP_SperateLength)))
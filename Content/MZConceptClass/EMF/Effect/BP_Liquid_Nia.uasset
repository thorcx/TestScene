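; BP_Liquid_Nia is an actor that drives a Niagara liquid effect through its separation and flow user parameters.
; The construction script pushes separation amount, force, position and length, plus life length and flow speed, from its variables to Niagara.
; Tick oscillates the separation with a sine of game time and re-applies it with the force.
; Pressing X plays a timeline that animates the flow speed.
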(event EventBeginPlay)

(event Collision|EventActorBeginOverlap
  (params (OtherActor :type Actor%20Object%20Reference)))

(event EventTick
  (params (DeltaSeconds :type Float%20%28single-precision%29))
  (Variables|Default|SetLiquidSperate (Math|Trig|Sin(Radians) (* (Utilities|Time|GetTimeSeconds) 3.0)))
  (CallFunction|UpdateSperate))

(event Input|KeyboardEvents|X
  (params (Key :type Key%20Structure))
  (:Pressed
    (bind _newtrack_0 (Timeline|Timeline_0 Play)
      (:Update
        (Niagara|SetNiagaraVariable(Float) (Variables|Default|GetNiagara) "User.FlowSpeed" _newtrack_0)))))

(fn ConstructionScript
  (CallFunction|UpdateSperate)
  (CallFunction|UpdatePosition)
  (CallFunction|UpdateSpeed))

(fn UpdateSperate
  (bind _niagara (Variables|Default|GetNiagara))
  (Niagara|SetNiagaraVariable(Float) _niagara "User.Sperate" (* (Variables|Default|GetLiquidSperate) 8e+01))
  (Niagara|SetNiagaraVariable(Float) _niagara "User.SperateForce" (Variables|Default|GetSperateForce)))

(fn UpdatePosition
  (bind _niagara (Variables|Default|GetNiagara))
  (Niagara|SetNiagaraVariable(Float) _niagara "User.SperatePosition" (Variables|Default|GetSperatePosition))
  (Niagara|SetNiagaraVariable(Float) _niagara "User.SperateLength" (Variables|Default|GetSperateLength))
  (Niagara|SetNiagaraVariable(Float) _niagara "User.LifeLength" (Variables|Default|GetLifeLength)))

(fn UpdateSpeed
  (Niagara|SetNiagaraVariable(Float) (Variables|Default|GetNiagara) "User.FlowSpeed" (Variables|Default|GetSpeed)))